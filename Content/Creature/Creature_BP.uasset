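; Creature Blueprint with a procedurally animated visual body that bobs in a bouncing motion.
; Tick accumulates delta time and feeds it through an absolute sine, scaled by an offset, to set the inner sphere's relative height.
; GetVisualBodyLocation returns that sphere's world location, so callers get the animated position.
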(event EventBeginPlay)

(event Collision|EventActorBeginOverlap
  (params (OtherActor :type Actor%20Object%20Reference)))

(event EventTick
  (params (DeltaSeconds :type Float%20%28single-precision%29))
  (bind _output_get (Variables|Default|SetBodyAnimValue (+ DeltaSeconds (Variables|Default|GetBodyAnimValue))))
  (Transformation|SetRelativeLocation (Variables|Default|GetInnerSphere) (Math|Vector|MakeVector 0.0 0.0 (* (Math|Float|Absolute(Float) (Math|Trig|Sin(Radians) _output_get)) (Variables|Default|GetBodyAnimOffset))) false false))

(fn ConstructionScript)

(fn GetVisualBodyLocation
  (return (Transformation|GetWorldLocation (Variables|Default|GetInnerSphere))))